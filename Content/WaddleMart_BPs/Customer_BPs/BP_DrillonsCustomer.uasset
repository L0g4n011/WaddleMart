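; BP_DrillonsCustomer is a customer character that walks to the Drillons register after a random wait.
; On BeginPlay it delays, then ToRegister finds the BP_DrillonsRegister actor and uses AI Move To toward it, stopping movement on arrival.
; Debug prints report each state.
; Queueing logic for stopping behind "Shopper"-tagged actors is disconnected, and the pawn-sensing, overlap and Tick events are empty.
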(event `self.ReceiveBeginPlay`
  ;[0.1459 0 0.15 0.5] Movement (Scrapped) (Maybe)
  (`KismetSystemLibrary.PrintString` "Waiting...")
  (`KismetSystemLibrary.Delay` (`KismetMathLibrary.RandomFloatInRange` 6.0 15.0))
  (`KismetSystemLibrary.PrintString` "Walking to Register...!")
  (`self.ToRegister`))

(event `ToRegister`
  ;[0.1459 0 0.15 0.5] Movement (Scrapped) (Maybe)
  ;;[0.03932 0.08694 0.15 0.5] Walk to Register
  (bind _returnvalue (`GameplayStatics.GetActorOfClass` "/Game/WaddleMart_BPs/Customer_BPs/BP_DrillonsRegister.BP_DrillonsRegister_C"))
  (`|AIMoveTo` self (`self.K2_GetActorLocation` _returnvalue) null 1.0
    (:`OnSuccess`
      (`KismetSystemLibrary.PrintString` "CUSTOMER REACHED REGISTER" true true (struct :`R` 0.188081 :`G` 1.0 :`A` 1.0))
      (`MovementComponent.StopMovementImmediately` (`self.CharacterMovement`)))
    (:`OnFail`
      (`KismetSystemLibrary.PrintString` "CUSTOMER CANNOT REACH REGISTER" true true (struct :`R` 1.0 :`B` 0.080471 :`A` 1.0)))))

(event `self.PawnSensing.OnSeePawn`
  (params (Pawn :type "Pawn Object Reference"))
  ;[0.1459 0 0.15 0.5] Movement (Scrapped) (Maybe)
  ;;[0.01727 0 0.15 0.5] Seeing other Customers
)

(fn `UserConstructionScript`)
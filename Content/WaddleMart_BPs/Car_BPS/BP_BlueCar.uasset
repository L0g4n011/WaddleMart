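; Blue car hazard that drives along a fixed path and knocks the first-person player away on contact.
; After a short delay on BeginPlay, a Timeline lerps the car from Start to End, then destroys the actor.
; Collision overlap enables physics on the player's capsule, launches them along their own forward vector, then calls their ragdoll check.
; An older overlap-polling version of the hit logic is left disconnected.
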(event `self.ReceiveBeginPlay`
  (`KismetSystemLibrary.Delay` 2.0)
  (bind (_direction _floattrack) (`Timeline|Timeline`)
    (:`Update`
      (`SceneComponent.K2_SetRelativeLocation` (`self.Car`) (`KismetMathLibrary.VLerp` (`SceneComponent.RelativeLocation` (`self.Start`)) (`SceneComponent.RelativeLocation` (`self.End`)) _floattrack) false false))
    (:`Finished`
      (`self.K2_DestroyActor`))))

(event `self.ReceiveTick`
  (params (DeltaSeconds :type "Float (single-precision)"))
  ; Checks if car collides with player and adds ragdoll physics
)

(event `self.Collision.OnComponentBeginOverlap`
  (params (OverlappedComponent :type "PrimitiveComponent Object Reference") (OtherActor :type "Actor Object Reference") (OtherComp :type "PrimitiveComponent Object Reference") (OtherBodyIndex :type Integer) (bFromSweep :type Boolean) (SweepResult :type "HitResult Structure (by ref)"))
  ; Checks Collison with car and player and adds physics and force to player
  (bind _asbp_first_person_character (cast `/Game/FirstPerson/Blueprints/BP_FirstPersonCharacter` OtherActor))
  (`PrimitiveComponent.SetSimulatePhysics` (`Character.CapsuleComponent` _asbp_first_person_character) true)
  (`Character.LaunchCharacter` _asbp_first_person_character (* (`KismetMathLibrary.GetForwardVector` (`SceneComponent.K2_GetComponentRotation` (`Actor.RootComponent` _asbp_first_person_character))) 5000.0) false false)
  (`KismetSystemLibrary.Delay` 0.1)
  (`KismetSystemLibrary.PrintString` "car hit you!")
  (bind _returnvalue (`GameplayStatics.GetActorOfClass` "/Game/FirstPerson/Blueprints/BP_FirstPersonCharacter.BP_FirstPersonCharacter_C"))
  (`/Game/FirstPerson/Blueprints/BP_FirstPersonCharacter.CheckifRagdollison` _asbp_first_person_character)
  (`/Game/FirstPerson/Blueprints/BP_FirstPersonCharacter.CheckifRagdollison` _returnvalue))

(fn `UserConstructionScript`)
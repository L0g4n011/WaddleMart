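; BP_CarManager is a car spawner manager that repeatedly spawns BP_BlueCar actors at BP_CarSpawner locations.
; On BeginPlay it gathers all spawners and calls SpawnCars, which loops over them, waits a random few seconds, spawns at the spawner's transform, then delays and calls itself again.
; Because the latent Delay sits inside the loop, each cycle effectively spawns one car at the last spawner.
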(event `self.ReceiveBeginPlay`
  (`KismetSystemLibrary.PrintString` "Car Spawner Works")
  (bind _outactors (`GameplayStatics.GetAllActorsOfClass` "/Game/WaddleMart_BPs/Car_BPS/BP_CarSpawner.BP_CarSpawner_C"))
  (set `self.Spawners` _outactors)
  (`self.Spawn Cars`))

(event `Spawn Cars`
  ;[0.1582 0.194 0.6198 0.5] Repeatedly Spawns Cars
  (for _array_element (`self.Spawners`)
    (`KismetSystemLibrary.Delay` (`KismetMathLibrary.Conv_IntToDouble` (`KismetMathLibrary.RandomIntegerInRange` 3 5)))
    (bind (_returnvalue_location _returnvalue_rotation) (`KismetMathLibrary.BreakTransform` (`SceneComponent.K2_GetComponentToWorld` (`/Game/WaddleMart_BPs/Car_BPS/BP_CarSpawner.DefaultSceneRoot` _array_element))))
    (`|SpawnActorFromClass` "/Game/WaddleMart_BPs/Car_BPS/BP_BlueCar.BP_BlueCar_C" (`KismetMathLibrary.MakeTransform` _returnvalue_location _returnvalue_rotation) "Undefined" "MultiplyWithRoot" null null)
    (`KismetSystemLibrary.Delay` 3.0)
    (`self.Spawn Cars`)))

(fn `UserConstructionScript`)
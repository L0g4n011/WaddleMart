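; BP_DialogueSystem is an NPC dialogue actor that shows conversations to the local player who last entered its sphere.
; Overlap toggles that player's input, and a debug E key or gamepad button opens W_Dialogue on their screen.
; GetNextLine reads data table rows to set text, portrait and sound, jumping to AnswerA on branches and closing at "end".
; A separate Talk event prints random lines and blanks a WB_Dialogue widget.
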(event OnComponentBeginOverlap(Sphere)
  (params (OverlappedComponent :type Primitive%20Component%20Object%20Reference) (OtherActor :type Actor%20Object%20Reference) (OtherComp :type Primitive%20Component%20Object%20Reference) (OtherBodyIndex :type Integer) (bFromSweep :type Boolean) (SweepResult :type Hit%20Result%20Structure%20%28by%20ref%29))
  (bind _asbp_first_person_character (Utilities|Casting|CastToBP_FirstPersonCharacter OtherActor))
  (Development|PrintString (Utilities|String|Append "Hello player " (Utilities|String|ToString(Integer) (+ (Variables|/Game/FirstPerson/Blueprints/BP_FirstPersonCharacter.BP_FirstPersonCharacter_C|GetPlayer%20Controller%20ID _asbp_first_person_character) 1)) "!"))
  (Input|EnableInput (Game|GetPlayerController (Variables|/Game/FirstPerson/Blueprints/BP_FirstPersonCharacter.BP_FirstPersonCharacter_C|GetPlayer%20Controller%20ID _asbp_first_person_character)))
  (Variables|Default|Setlast%20touched%20Player%20ID (Variables|/Game/FirstPerson/Blueprints/BP_FirstPersonCharacter.BP_FirstPersonCharacter_C|GetPlayer%20Controller%20ID _asbp_first_person_character))
  (Development|PrintString "press E to start dialogue"))

(event OnComponentEndOverlap(Sphere)
  (params (OverlappedComponent :type Primitive%20Component%20Object%20Reference) (OtherActor :type Actor%20Object%20Reference) (OtherComp :type Primitive%20Component%20Object%20Reference) (OtherBodyIndex :type Integer))
  (Utilities|Casting|CastToBP_FirstPersonCharacter OtherActor)
  (Input|DisableInput (Game|GetPlayerController (Variables|Default|Getlast%20touched%20Player%20ID)))
  (Widget|RemovefromParent (Variables|Default|Getdialog%20widget)) ; remove the widget
)

(event Custom|Get%20Next%20Line
  (bind _outrownames (DataTable|GetDataTableRowNames "/Game/WaddleMart_BPs/Dialogue_BPs/DataForDialogue/dialogueTest_-_dialogueTest_csv.dialogueTest_-_dialogueTest_csv"))
  (bind _returnvalue (Utilities|GetDataTableRow "/Game/WaddleMart_BPs/Dialogue_BPs/DataForDialogue/DT_Dialogue.DT_Dialogue" (Utilities|Array|Get(acopy) _outrownames (Variables|Default|Getdialogueindex)))
    (:then
      (if (Utilities|Enum|Equal(Enum) (.text _returnvalue) "end") ; if this is true, stop the widget
        (Widget|RemovefromParent (Variables|Default|Getdialog%20widget))
        (else
          (Rendering|Components|TextRender|SetText (Variables|/Game/UI/W_Dialogue.W_Dialogue_C|GetNPCTextBlock (Variables|Default|Getdialog%20widget)) (Utilities|Text|ToText(String) (.text _returnvalue)))
          (Appearance|SetBrushfromTexture (Variables|/Game/UI/W_Dialogue.W_Dialogue_C|GetNPCImage (Variables|Default|Getdialog%20widget)) (Utilities|Select :Index (.speaker _returnvalue) :Option%200 0 :Option%201 0 :Option%202 0 :Option%203 0 :Option%204 0) false)
          (Audio|PlaySoundatLocation 0 (Transformation|GetWorldLocation (Variables|Default|GetSkeletalMesh)) "0, 0, 0" 1.0 1.0 0.0 0 0 0 0)
          (if (.branchable _returnvalue) ; Is this a branch?
            (Variables|Default|SetdialogueIndex (.answera _returnvalue))
            (else
              (Math|Integer|IncrementInt (Variables|Default|GetdialogueIndex)))))))))

(event EventBeginPlay)

(event EventTalk
  (bind _output_get (Variables|Default|SettalkIndex (Math|Random|RandomIntegerinRange 0 6)))
  (Development|PrintString (Utilities|Array|Get(acopy) (Variables|Default|GetDialogue) _output_get))
  (Variables|Default|GetUI
    (:then
      _)
    (:else
      (bind _returnvalue (UserInterface|CreateWidget "/Game/WaddleMart_BPs/Dialogue_BPs/WB_Dialogue.WB_Dialogue_C" (Game|GetPlayerController 0)))
      (bind _output_get_2 (Variables|Default|SetUI _returnvalue))
      (UserInterface|Viewport|AddtoPlayerScreen _output_get_2)))
  (Rendering|Components|TextRender|SetText (Variables|/Game/WaddleMart_BPs/Dialogue_BPs/WB_Dialogue.WB_Dialogue_C|GetDialogue (Variables|Default|GetUI)) ""))

(event Input|KeyboardEvents|DebugKeyE
  (params (Key :type Key%20Structure :default "None") (ActionValue :type Input%20Action%20Value%20Structure))
  ;[0.15 0 0 0.5] Replace this with an input event
  (:Pressed
    (Utilities|IsValid (Variables|Default|Getdialog%20widget) ; Do we already have a dialogue widget?\nThen show that one.\nOtherwise, create a new dialogue widget!
      (:Is%20Valid
        _)
      (:Is%20Not%20Valid
        (bind _returnvalue (UserInterface|CreateWidget "/Game/UI/W_Dialogue.W_Dialogue_C" (Game|GetPlayerController (Variables|Default|Getlast%20touched%20Player%20ID))))
        (Variables|Default|Setdialog%20widget _returnvalue)))
    (UserInterface|Viewport|AddtoPlayerScreen (Variables|Default|Getdialog%20widget))))

(event Input|GamepadEvents|GamepadFaceButtonLeft
  (params (Key :type Key%20Structure :default "None"))
  ;[0.15 0 0 0.5] Replace this with an input event
  (:Pressed
    (Utilities|IsValid (Variables|Default|Getdialog%20widget) ; Do we already have a dialogue widget?\nThen show that one.\nOtherwise, create a new dialogue widget!
      (:Is%20Valid
        _)
      (:Is%20Not%20Valid
        (bind _returnvalue (UserInterface|CreateWidget "/Game/UI/W_Dialogue.W_Dialogue_C" (Game|GetPlayerController (Variables|Default|Getlast%20touched%20Player%20ID))))
        (Variables|Default|Setdialog%20widget _returnvalue)))
    (UserInterface|Viewport|AddtoPlayerScreen (Variables|Default|Getdialog%20widget))))

(fn ConstructionScript)
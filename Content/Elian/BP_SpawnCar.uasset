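; BP_SpawnCar spawns a BP_Car actor on BeginPlay and moves a car mesh along a spline.
; SpawnCar takes the spawn transform from the existing Car reference, stores the new actor there, assigns the BlueCar mesh and applies the Scale transform.
; A successful transform sets Success, which lets Tick advance a distance by Speed and place CarMesh at that spline point.
; Debug prints report the spawn outcome.
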(event `self.ReceiveBeginPlay`
  (`self.SpawnCar`))

(event `self.ReceiveTick`
  (params (DeltaSeconds :type "Float (single-precision)"))
  (if (`self.Success`)
    (bind _output_get (set `self.Position` (+ (* DeltaSeconds (`self.speed`)) (`self.Position`))))
    (`SceneComponent.K2_SetWorldTransform` (`self.CarMesh`) (`SplineComponent.GetTransformAtDistanceAlongSpline` (`self.Spline`) _output_get "World" false) false false)))

(fn `SpawnCar`
  (bind _returnvalue (`|SpawnActorFromClass` "/Game/Elian/BP_Car.BP_Car_C" (`self.GetTransform` (`self.Car`)) "Undefined" "MultiplyWithRoot" null null))
  (bind _output_get (set `self.Car` _returnvalue))
  (`StaticMeshComponent.SetStaticMesh` (`/Game/Elian/BP_Car.idk` _output_get) "/Game/Fab/Cars/BlueCar.BlueCar")
  (bind (_sweephitresult _returnvalue_2) (`self.K2_SetActorTransform` (`self.Car`) (`self.Scale`) false false))
  (if _returnvalue_2
    (set `self.success` true)
    (`KismetSystemLibrary.PrintString` "car!")
    (else
      (`KismetSystemLibrary.PrintString` "No car :("))))

(fn `UserConstructionScript`)